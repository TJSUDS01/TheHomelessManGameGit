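; Character component that adds a momentum-based crouch slide to its owning Character.
; StartSliding checks a speed threshold, then crouches, launches the character forward, lowers friction, braking and acceleration, and sets a timed stop.
; While sliding, Tick adds gravity force projected onto the floor plane, or small horizontal launches along velocity when airborne.
; Stopping uncrouches and writes back hardcoded movement values rather than cached originals.
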(event `self.ReceiveBeginPlay`
  ; start sliding
  (bind _ascharacter (cast `Character` (`self.GetOwner`)))
  (bind _output_get (set `self.As Character` _ascharacter))
  (set `self.Character Movement` (`Character.CharacterMovement` _output_get)))

(event `Start Sliding`
  (bind _as_character (`self.As Character`))
  (bind _character_movement (`self.Character Movement`))
  ; start sliding
  (if (> (`KismetMathLibrary.VSize` (`MovementComponent.Velocity` (`self.Character Movement`))) (`self.slide speed threshold`))
    (set `self.Is sliding?` true)
    (`Character.Crouch` _as_character)
    (`Character.LaunchCharacter` _as_character (* (`Actor.GetActorForwardVector` _as_character) (`self.slide impulse`)) false false)
    (set `CharacterMovementComponent.GroundFriction` 0.05 _character_movement)
    (set `CharacterMovementComponent.BrakingDecelerationWalking` 10.0 _character_movement)
    (set `CharacterMovementComponent.MaxWalkSpeedCrouched` 1200.0 _character_movement)
    (set `CharacterMovementComponent.MaxAcceleration` 0.0 _character_movement)
    (set `CharacterMovementComponent.bOrientRotationToMovement` false _character_movement)
    (set `Pawn.bUseControllerRotationYaw` true (`self.As Character`))
    (`KismetSystemLibrary.K2_SetTimer` null "stop sliding" 3.0)
    (else
      (`Character.UnCrouch` (`self.As Character`)))))

(event `stop sliding`
  (bind _character_movement (`self.Character Movement`))
  ; stop sliding
  (set `self.Is sliding?` false)
  (`Character.UnCrouch` (`self.As Character`))
  (set `CharacterMovementComponent.GroundFriction` 8.0 _character_movement)
  (set `CharacterMovementComponent.BrakingDecelerationWalking` 2048.0 _character_movement)
  (set `CharacterMovementComponent.MaxWalkSpeedCrouched` 300.0 _character_movement)
  (set `CharacterMovementComponent.MaxAcceleration` 2048.0 _character_movement)
  (set `CharacterMovementComponent.bOrientRotationToMovement` true _character_movement)
  (set `Pawn.bUseControllerRotationYaw` true (`self.As Character`))
  (`KismetSystemLibrary.K2_ClearTimer` null "stop sliding"))

(event `self.ReceiveTick`
  (params (DeltaSeconds :type "Float (single-precision)"))
  (bind _as_character (`self.As Character`))
  (bind (_returnvalue_x _returnvalue_y) (`KismetMathLibrary.BreakVector` (`Actor.GetVelocity` _as_character)))
  ; force of slide
  (if (`self.Is sliding?`)
    (if (not (`NavMovementComponent.IsFalling` (`self.Character Movement`)))
      (`CharacterMovementComponent.AddForce` (`self.Character Movement`) (* (`KismetMathLibrary.ProjectVectorOnToPlane` (`KismetMathLibrary.MakeVector` 0.0 0.0 -1.0) (`.ImpactNormal` (`GameplayStatics.BreakHitResult` (`.HitResult` (break `FindFloorResult` (`CharacterMovementComponent.CurrentFloor` (`self.Character Movement`))))))) (`self.Slide Gravity Force`)))
      (else
        ;; launch character
        (`Character.LaunchCharacter` _as_character (* (`KismetMathLibrary.Normal` (`KismetMathLibrary.MakeVector` _returnvalue_x _returnvalue_y)) 15.0) false false)))))