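; AI camera Blueprint that keeps its Arrow component turning to face player character 0.
; Each Tick it computes a look-at rotation from the arrow to the player and eases the arrow's world rotation toward it with RInterpTo.
; The DeltaTime and InterpSpeed inputs are swapped, with a constant as delta time and world delta seconds as speed.
; The construction script is empty.
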(event `self.ReceiveTick`
  (params (DeltaSeconds :type "Float (single-precision)"))
  (`SceneComponent.K2_SetWorldRotation` (`self.Arrow`) (`KismetMathLibrary.RInterpTo` (`SceneComponent.K2_GetComponentRotation` (`self.Arrow`)) (`KismetMathLibrary.FindLookAtRotation` (`SceneComponent.K2_GetComponentLocation` (`self.Arrow`)) (`self.K2_GetActorLocation` (`GameplayStatics.GetPlayerCharacter` 0))) 5.0 (`GameplayStatics.GetWorldDeltaSeconds`)) false false))

(fn `UserConstructionScript`)