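; BP_Enemy is a melee enemy that roams randomly until AI Perception senses the first-person player, then chases and attacks.
; Roaming loops AIMoveTo to random reachable points at walk speed; detection shows an alert, plays a sound and raises speed.
; On reaching the player it plays a baton montage, applies damage through BPC_DamageSystem and repeats while chasing.
; It binds itself to a healthbar widget, but its own health and damage functions are empty stubs.
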(event `Random Roam`
  ;[0.07907 0.75 0.1984 0.5] Roaming (Patrol /Random Movemnet)
  (if (not (`self.IsChasing`))
    (set `CharacterMovementComponent.MaxWalkSpeed` 150.0 (`self.CharacterMovement`))
    (`|AIMoveTo` self (`NavigationSystemV1.K2_GetRandomReachablePointInRadius` (`self.K2_GetActorLocation`) 1000.0 null null) null 100.0
      (:`OnSuccess`
        _)
      (:`OnFail`
        _))
    (`KismetSystemLibrary.Delay` (`KismetMathLibrary.RandomFloatInRange` 0.1 0.2))
    (`self.Random Roam`)))

(event `self.ReceiveBeginPlay`
  ;[0.1727 0.1763 0.8438 0.5] Player Detection (AI Perception)
  (`|ExecutionSequence`
    (:`then_0`
      (add `AIPerceptionComponent.OnTargetPerceptionUpdated` (`self.AIPerception`) (delegate `OnTargetPerceptionUpdated_Event`))
      (`self.Random Roam`))
    (:`then_1`
      (bind _asw_healthbar (cast `/Game/tjs/health/W_Healthbar` (`WidgetComponent.GetUserWidgetObject` (`self.Widget`))))
      (set `/Game/tjs/health/W_Healthbar.Damageable Actor` self _asw_healthbar))))

(event `OnTargetPerceptionUpdated_Event`
  (params (Actor :type "Actor Object Reference") (Stimulus :type "AIStimulus Structure"))
  (bind _returnvalue (`GameplayStatics.GetPlayerCharacter` 0))
  (bind _detectionalert (`self.DetectionAlert`))
  ;[0.1727 0.1763 0.8438 0.5] Player Detection (AI Perception)
  (bind _asbp_first_person_character (cast `/Game/FirstPerson/Blueprints/BP_FirstPersonCharacter` Actor))
  (if (`.bSuccessfullySensed` (break `AIStimulus` Stimulus))
    (set `self.IsChasing` true)
    (`SceneComponent.SetVisibility` _detectionalert true false)
    (`GameplayStatics.PlaySound2D` "/Game/AI/Noises/SFX_SecurityDetected.SFX_SecurityDetected" 1.0 1.0 0.0 null null)
    ;[0.7396 0.4006 0 0.5] Chasing(Pursue Player)
    (set `CharacterMovementComponent.MaxWalkSpeed` 450.0 (`self.CharacterMovement`) :!label _label)
    (`|AIMoveTo` self (0.0 0.0 0.0) _asbp_first_person_character 80.0 true
      (:`OnSuccess`
        (`self.K2_SetActorRotation` (`KismetMathLibrary.FindLookAtRotation` (`self.K2_GetActorLocation`) (`self.K2_GetActorLocation` _returnvalue)))
        (`self.PlayAnimMontage` "/Game/AI/Animations/AM_BatonAttack.AM_BatonAttack" 1.3)
        ;[0.9583 0.03297 0 0.5] Attacking (Deal Damage)
        (`/Game/tjs/DamageSystem/BPC_DamageSystem.TakeDamage` (`self.GetComponentByClass` _returnvalue "/Game/tjs/DamageSystem/BPC_DamageSystem.BPC_DamageSystem_C") (make `/Game/tjs/DamageSystem/S_DamageInfo` 10.0))
        (`KismetSystemLibrary.Delay` 1.8)
        (if (`self.IsChasing`)
          (`KismetSystemLibrary.PrintString` "Damage")
          (goto _label))))
    (else
      (set `self.IsChasing` false)
      (`SceneComponent.SetVisibility` _detectionalert false false)
      (`self.Random Roam`))))

(fn `GetCurrentHealth`
  (returns (Health :type "Float (double-precision)"))
  (return 0.0))

(fn `GetMaxHealth`
  (returns (MaxHealth :type "Float (double-precision)"))
  (return 0.0))

(fn `Heal`
  (params (Amount :type "Float (double-precision)"))
  (returns (NewHealth :type "Float (double-precision)"))
  (return 0.0))

(fn `TakeDamage`
  (params (DamageInfo :type "/Game/tjs/DamageSystem/S_DamageInfo Structure"))
  (returns (WasDamaged :type Boolean))
  (return false))

(fn `UserConstructionScript`)